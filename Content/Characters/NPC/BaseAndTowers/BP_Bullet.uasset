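; BP_Bullet is a homing projectile that damages and applies an effect to BP_Enemy actors.
; Each Tick it turns toward its Target and steps forward by Speed without delta-time scaling, destroying itself if the target is no longer valid.
; When its sphere overlaps any BP_Enemy, it applies its Effect and Damage, then calls a custom Destroy that spawns a small explosion emitter before removing the actor.
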(event OnComponentBeginOverlap(Sphere)
  (params (OverlappedComponent :type Primitive%20Component%20Object%20Reference) (OtherActor :type Actor%20Object%20Reference) (OtherComp :type Primitive%20Component%20Object%20Reference) (OtherBodyIndex :type Integer) (bFromSweep :type Boolean) (SweepResult :type Hit%20Result%20Structure%20%28by%20ref%29))
  (bind _asbp_enemy (Utilities|Casting|CastToBP_Enemy OtherActor))
  (Default|ApplyEffect _asbp_enemy (Variables|Default|GetEffect))
  (Game|Damage|ApplyDamage _asbp_enemy (Variables|Default|GetDamage) 0 0)
  (CallFunction|Destroy))

(event EventTick
  (params (DeltaSeconds :type Float%20%28single-precision%29))
  (bind _target (Variables|Default|GetTarget)
    (:then
      (Transformation|SetActorTransform (Math|Transform|MakeTransform (+ (Transformation|GetActorLocation) (* (Math|Vector|GetForwardVector (Math|Rotator|FindLookatRotation (Transformation|GetActorLocation) (.location (Transformation|GetActorTransform _target)))) (Variables|Default|GetSpeed))) (Math|Rotator|FindLookatRotation (Transformation|GetActorLocation) (.location (Transformation|GetActorTransform _target))) "1.000000,1.000000,1.000000")))
    (:else
      (CallFunction|Destroy))))

(fn ConstructionScript)

(fn Destroy
  (Effects|SpawnEmitteratLocation "/Game/StarterContent/Particles/P_Explosion.P_Explosion" (Transformation|GetActorLocation) "0, 0, 0" "0.040000,0.040000,0.040000")
  (Actor|DestroyActor))