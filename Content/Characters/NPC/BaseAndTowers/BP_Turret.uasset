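; BP_Turret is a tower that automatically shoots BP_Enemy actors inside a sphere sized by its TurretStats.
; Overlap events maintain the enemy list and re-pick the target with the least distance left, only on enter or exit.
; Tick yaws toward the target and uses a Delay to pace shots, spawning stat-driven BP_Bullets from alternating barrels.
; Each shot spawns a small explosion effect and plays a timeline recoil that scales the barrel.
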(event OnComponentBeginOverlap(Sphere)
  (params (OverlappedComponent :type Primitive%20Component%20Object%20Reference) (OtherActor :type Actor%20Object%20Reference) (OtherComp :type Primitive%20Component%20Object%20Reference) (OtherBodyIndex :type Integer) (bFromSweep :type Boolean) (SweepResult :type Hit%20Result%20Structure%20%28by%20ref%29))
  (bind _asbp_enemy (Utilities|Casting|CastToBP_Enemy OtherActor))
  (Utilities|Array|Add (Variables|Default|GetAviableEnemies) _asbp_enemy)
  (CallFunction|UpdateTarget))

(event OnComponentEndOverlap(Sphere)
  (params (OverlappedComponent :type Primitive%20Component%20Object%20Reference) (OtherActor :type Actor%20Object%20Reference) (OtherComp :type Primitive%20Component%20Object%20Reference) (OtherBodyIndex :type Integer))
  (bind _aviableenemies (Variables|Default|GetAviableEnemies))
  (bind _asbp_enemy (Utilities|Casting|CastToBP_Enemy OtherActor))
  (Utilities|Array|RemoveItem _aviableenemies _asbp_enemy)
  (if (== (Utilities|Array|FindItem _aviableenemies (Variables|Default|GetTarget)) -1)
    (Variables|Default|SetTarget 0))
  (CallFunction|UpdateTarget))

(event EventBeginPlay
  (Components|Sphere|SetSphereRadius (Variables|Default|GetSphere) (.radius (Variables|Default|GetTurretStats)) true)
  (Variables|Default|SetBarrelScale (Transformation|GetWorldScale (Variables|Default|GetBarrel1))))

(event EventTick
  (params (DeltaSeconds :type Float%20%28single-precision%29))
  (bind _turretstats (Variables|Default|GetTurretStats))
  (bind _barrelscale (Variables|Default|GetBarrelScale))
  (bind _barrelscale_2 (Variables|Default|GetBarrelScale))
  (bind _target (Variables|Default|GetTarget)
    (:then
      (Transformation|SetActorRotation (Math|Rotator|MakeRotator 0.0 0.0 (.yaw (Math|Rotator|FindLookatRotation (Transformation|GetActorLocation) (.location (Transformation|GetActorTransform _target))))))
      (Utilities|FlowControl|Delay (.speed (Variables|Default|GetTurretStats)))
      ;[1 1 1] shot
      (Variables|Default|SetIsBarrel1 (not (Variables|Default|GetIsBarrel1)))
      (Game|SpawnActorfromClass "/Game/Characters/NPC/BaseAndTowers/BP_Bullet.BP_Bullet_C" (Math|Transform|MakeTransform (select (Variables|Default|GetIsBarrel1) (Transformation|GetSocketLocation (Variables|Default|GetBulletHole1) "1") (Transformation|GetSocketLocation (Variables|Default|GetBulletHole2) "2")) "0, 0, 0" "1.000000,1.000000,1.000000") "Undefined" "OverrideRootScale" 0 (.damage _turretstats) (.bulletspeed _turretstats) (Variables|Default|GetTarget) (.effect _turretstats) 0)
      (Effects|SpawnEmitteratLocation "/Game/StarterContent/Particles/P_Explosion.P_Explosion" (select (Variables|Default|GetIsBarrel1) (Transformation|GetSocketLocation (Variables|Default|GetBulletHole1) "1") (Transformation|GetSocketLocation (Variables|Default|GetBulletHole2) "2")) "0, 0, 0" "0.080000,0.080000,0.080000")
      (Components|Timeline|SetPlayRate (Variables|Default|GetRecoil) (/ 1.0 (.speed (Variables|Default|GetTurretStats))))
      (if (Variables|Default|GetIsBarrel1)
        (bind _alpha (Timeline|Recoil PlayFromStart)
          (:Update
            (Transformation|SetWorldScale3D (Variables|Default|GetBarrel1) (Math|Vector|MakeVector (.x _barrelscale_2) (.y _barrelscale_2) (Math|Float|Lerp (/ (.z _barrelscale_2) 2.0) (.z _barrelscale_2) _alpha)))))
        (else
          (bind _alpha_2 (Timeline|Recoil2 PlayFromStart)
            (:Update
              (Transformation|SetWorldScale3D (Variables|Default|GetBarrel2) (Math|Vector|MakeVector (.x _barrelscale) (.y _barrelscale) (Math|Float|Lerp (/ (.z _barrelscale) 2.0) (.z _barrelscale) _alpha_2))))))))
    (:else)))

(fn ConstructionScript)

(fn UpdateTarget
  (for _array_element (Variables|Default|GetAviableEnemies)
    (bind _target (Variables|Default|GetTarget)
      (:then
        (if (< (Utilities|DistanceLeft _array_element) (Utilities|DistanceLeft _target))
          (Variables|Default|SetTarget _array_element :!label _label)))
      (:else
        (goto _label)))))