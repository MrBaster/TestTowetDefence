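; BP_PlatformTurret is a turret platform where the player builds or destroys a single turret.
; Capsule overlap by BP_ThirdPersonCharacter toggles a HUD hint and a range indicator scaled from the placed turret's radius, or the player's selected turret's when empty.
; Interact spawns the player's CurrentTurret or destroys the existing one, swaps the platform material, then refreshes hint and radius.
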(event OnComponentBeginOverlap(Capsule)
  (params (OverlappedComponent :type Primitive%20Component%20Object%20Reference) (OtherActor :type Actor%20Object%20Reference) (OtherComp :type Primitive%20Component%20Object%20Reference) (OtherBodyIndex :type Integer) (bFromSweep :type Boolean) (SweepResult :type Hit%20Result%20Structure%20%28by%20ref%29))
  (Utilities|Casting|CastToBP_ThirdPersonCharacter OtherActor)
  (CallFunction|UpdateHint true)
  (Rendering|SetVisibility (Variables|Default|GetRadius) true false)
  (CallFunction|UpdateRadius))

(event OnComponentEndOverlap(Capsule)
  (params (OverlappedComponent :type Primitive%20Component%20Object%20Reference) (OtherActor :type Actor%20Object%20Reference) (OtherComp :type Primitive%20Component%20Object%20Reference) (OtherBodyIndex :type Integer))
  (Utilities|Casting|CastToBP_ThirdPersonCharacter OtherActor)
  (CallFunction|UpdateHint false)
  (Rendering|SetVisibility (Variables|Default|GetRadius) false false))

(event EventBeginPlay)

(event Collision|EventActorBeginOverlap
  (params (OtherActor :type Actor%20Object%20Reference)))

(event EventTick
  (params (DeltaSeconds :type Float%20%28single-precision%29)))

(fn ConstructionScript)

(fn UpdateRadius
  (bind _player (CallFunction|GetPlayer))
  (bind _radius (Variables|Default|GetRadius))
  (bind _turret (Variables|Default|GetTurret))
  (bind _turret_2 (Variables|Default|GetTurret))
  (bind _returnvalue (Transformation|GetWorldTransform _radius))
  (bind _returnvalue_2 (Utilities|IsValid _turret_2))
  (bind _currentturret (Variables|/Game/ThirdPerson/Blueprints/BP_ThirdPersonCharacter.BP_ThirdPersonCharacter_C|GetCurrentTurret _player))
  (bind _turretstats (Variables|/Game/Characters/NPC/BaseAndTowers/BP_Turret.BP_Turret_C|GetTurretStats _turret))
  (bind _returnvalue_3 (select _returnvalue_2 (.radius _turretstats) (.radius _currentturret)))
  (bind _returnvalue_4 (/ _returnvalue_3 5e+01))
  (Transformation|SetWorldTransform _radius (Math|Transform|MakeTransform (.location _returnvalue) (.rotation _returnvalue) (Math|Vector|MakeVector _returnvalue_4 _returnvalue_4 _returnvalue_4)) false false))

(fn UpdateHint
  (params (IsVisible :type Boolean))
  (bind _asbp_third_person_character (Utilities|Casting|CastToBP_ThirdPersonCharacter (Game|Player|GetPlayerPawn 0)))
  (Default|UpdateHint (Variables|/Game/ThirdPerson/Blueprints/BP_ThirdPersonCharacter.BP_ThirdPersonCharacter_C|GetHUD _asbp_third_person_character) (select (Utilities|IsValid (Variables|Default|GetTurret)) "\"E\" to Destroy" (Variables|Default|GetHintText)) IsVisible))

(fn Interact
  (bind _player (CallFunction|GetPlayer))
  (bind _returnvalue (Transformation|GetActorTransform))
  (Variables|Default|GetTurret
    (:then
      (Rendering|Material|SetMaterial (Variables|Default|GetPlatrorm) 0 "/Game/StarterContent/Materials/M_Tech_Hex_Tile.M_Tech_Hex_Tile")
      (Actor|DestroyActor (Variables|Default|GetTurret))
      (Variables|Default|SetTurret 0))
    (:else
      (Rendering|Material|SetMaterial (Variables|Default|GetPlatrorm) 0 "/Game/StarterContent/Materials/M_Tech_Hex_Tile_Pulse.M_Tech_Hex_Tile_Pulse")
      (bind _returnvalue_2 (Game|SpawnActorfromClass (.class (Variables|/Game/ThirdPerson/Blueprints/BP_ThirdPersonCharacter.BP_ThirdPersonCharacter_C|GetCurrentTurret _player)) (Math|Transform|MakeTransform (Math|Vector|MakeVector (.x (.location _returnvalue)) (.y (.location _returnvalue)) 0.0) (.rotation _returnvalue) (.scale _returnvalue)) "Undefined" 0 (Variables|/Game/ThirdPerson/Blueprints/BP_ThirdPersonCharacter.BP_ThirdPersonCharacter_C|GetCurrentTurret _player) 0))
      (Variables|Default|SetTurret _returnvalue_2)))
  (CallFunction|UpdateHint true)
  (CallFunction|UpdateRadius)
  (return true))