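; BP_Enemy is an enemy that follows a spline path, damages the player's base on arrival, then destroys itself.
; The MoveEnemy timeline drives position, with play rate set by speed and path time.
; Timers run Frost, which alters that rate temporarily, and looping Fire damage, though the fire tick limit clears FrostTimer, not FireTimer.
; Damage updates a color-lerped health bar and triggers an explosion and destruction at zero HP.
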(event Custom|Move
  (Components|Timeline|SetPlayRate (Variables|Default|GetMoveEnemy) (* (/ 1.0 (Variables|Default|GetPathTime)) (.speed (Variables|Default|GetSEnemyStats))))
  (bind _pathpoint (Timeline|MoveEnemy Play)
    (:Update
      (Variables|Default|SetCurrentDistance (Math|Float|Lerp 0.0 (Spline|GetSplineLength (Utilities|GetSpline)) _pathpoint))
      (Variables|Default|SetCurrentDistancePercent _pathpoint)
      (Transformation|SetActorTransform (Spline|GetTransformatDistanceAlongSpline (Utilities|GetSpline) (Math|Float|Lerp 0.0 (Spline|GetSplineLength (Utilities|GetSpline)) _pathpoint) "World" false)))
    (:Finished
      (CallFunction|Finish))))

(event Custom|ApplyEffect
  (params (Effect :type EnumTurretEffect%20Enum :default "NewEnumerator0"))
  ;[1 1 1] Effect
  (switch Utilities|FlowControl|Switch|SwitchonEnumTurretEffect Effect
    (:NewEnumerator1
      ;;[1 1 1] Frost
      (Components|Timeline|SetPlayRate (Variables|Default|GetMoveEnemy) (* (/ 1.0 (* (Variables|Default|GetPathTime) (Variables|Frost|GetFrostPower))) (.speed (Variables|Default|GetSEnemyStats))))
      (Utilities|Time|ClearandInvalidateTimerbyHandle (Variables|Frost|GetFrostTimer))
      (bind _returnvalue (Utilities|Time|SetTimerbyEvent (delegate Custom|Unfrost) (Variables|Frost|GetFrostTime)))
      (Variables|Frost|SetFrostTimer _returnvalue))
    (:NewEnumerator2
      (bind _returnvalue_2 (Utilities|Time|SetTimerbyEvent (delegate Custom|FireTick) (Variables|Fire|GetFireTickRate) true))
      (Variables|Frost|SetFireTimer _returnvalue_2))))

(event Custom|Unfrost
  ;[1 1 1] Effect
  ;;[1 1 1] Frost
  (Components|Timeline|SetPlayRate (Variables|Default|GetMoveEnemy) (* (/ 1.0 (Variables|Default|GetPathTime)) (.speed (Variables|Default|GetSEnemyStats)))))

(event Custom|FireTick
  (bind _currentfiretick (Variables|Fire|GetCurrentFireTick))
  ;[1 1 1] Effect
  (Game|Damage|ApplyDamage self (Variables|Fire|GetFireDamage) 0 0)
  (Math|Float|IncrementFloat _currentfiretick
    (:%20%20
      (if (>= _currentfiretick (Variables|Fire|GetFireTickDuration))
        (Utilities|Time|ClearandInvalidateTimerbyHandle (Variables|Frost|GetFrostTimer))))))

(event EventBeginPlay
  (CallFunction|Move)
  (Variables|Default|SetCurrentHP (.hp (Variables|Default|GetSEnemyStats)))
  (CallFunction|UpdateHealthBar))

(event Game|Damage|EventAnyDamage
  (params (Damage :type Float%20%28single-precision%29) (DamageType :type Damage%20Type%20Object%20Reference) (InstigatedBy :type Controller%20Object%20Reference) (DamageCauser :type Actor%20Object%20Reference))
  (bind _output_get (Variables|Default|SetCurrentHP (- (Variables|Default|GetCurrentHP) Damage)))
  (CallFunction|UpdateHealthBar)
  (if (<= _output_get 0.0)
    (CallFunction|Death)))

(fn ConstructionScript)

(fn Finish
  (Default|BaseDamage (CallFunction|GetPlayer))
  (Actor|DestroyActor))

(fn Death
  (Effects|SpawnEmitteratLocation "/Game/StarterContent/Particles/P_Explosion.P_Explosion" (Transformation|GetActorLocation))
  (Actor|DestroyActor))

(fn UpdateHealthBar
  (bind _currenthp (Variables|Default|GetCurrentHP))
  (bind _senemystats (Variables|Default|GetSEnemyStats))
  (bind _returnvalue (/ _currenthp (.hp _senemystats)))
  (bind _aswb_hpbar (Utilities|Casting|CastToWB_HPBar (UserInterface|GetUserWidgetObject (Variables|Default|GetHPBar))))
  (Variables|/Game/Characters/NPC/Enemies/WB_HPBar.WB_HPBar_C|SetHPPBHealth _aswb_hpbar _returnvalue)
  (Variables|/Game/Characters/NPC/Enemies/WB_HPBar.WB_HPBar_C|SetHPPBColor _aswb_hpbar (Math|Color|Lerp(LinearColor) "(R=1.000000,G=0.009895,B=0.000000,A=1.000000)" "(R=0.013265,G=1.000000,B=0.000000,A=1.000000)" _returnvalue)))